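; BP_TurretGhost is a turret preview that signals whether its spot is clear of enemies for spawning.
; When a BP_BaseEnemy enters its Box, it clears IsSpawn and switches the Platform, Gun and Rack meshes to the invalid ghost material.
; An enemy leaving sets IsSpawn and restores the valid material, without checking for other enemies still inside.
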(event `self.Box.OnComponentBeginOverlap`
  (params (OverlappedComponent :type "PrimitiveComponent Object Reference") (OtherActor :type "Actor Object Reference") (OtherComp :type "PrimitiveComponent Object Reference") (OtherBodyIndex :type Integer) (bFromSweep :type Boolean) (SweepResult :type "HitResult Structure (by ref)"))
  (cast `/Game/Content/Blueprints/BP_BaseEnemy` OtherActor)
  (set `self.bIsSpawn` false)
  (`|ExecutionSequence`
    (:`then_0`
      (`PrimitiveComponent.SetMaterial` (`self.Platform`) 0 "/Game/Content/Blueprints/Materials/MI_GhostMeshFalse.MI_GhostMeshFalse"))
    (:`then_1`
      (`PrimitiveComponent.SetMaterial` (`self.Gun`) 0 "/Game/Content/Blueprints/Materials/MI_GhostMeshFalse.MI_GhostMeshFalse"))
    (:`then_2`
      (`PrimitiveComponent.SetMaterial` (`self.Rack`) 0 "/Game/Content/Blueprints/Materials/MI_GhostMeshFalse.MI_GhostMeshFalse"))))

(event `self.Box.OnComponentEndOverlap`
  (params (OverlappedComponent :type "PrimitiveComponent Object Reference") (OtherActor :type "Actor Object Reference") (OtherComp :type "PrimitiveComponent Object Reference") (OtherBodyIndex :type Integer))
  (cast `/Game/Content/Blueprints/BP_BaseEnemy` OtherActor)
  (set `self.bIsSpawn` true)
  (`|ExecutionSequence`
    (:`then_0`
      (`PrimitiveComponent.SetMaterial` (`self.Platform`) 0 "/Game/Content/Blueprints/Materials/MI_GhostMeshTrue.MI_GhostMeshTrue"))
    (:`then_1`
      (`PrimitiveComponent.SetMaterial` (`self.Gun`) 0 "/Game/Content/Blueprints/Materials/MI_GhostMeshTrue.MI_GhostMeshTrue"))
    (:`then_2`
      (`PrimitiveComponent.SetMaterial` (`self.Rack`) 0 "/Game/Content/Blueprints/Materials/MI_GhostMeshTrue.MI_GhostMeshTrue"))))

(fn `UserConstructionScript`)