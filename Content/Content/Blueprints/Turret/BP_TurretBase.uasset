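; Base turret actor that sweeps its gun's yaw with a timeline and damages enemies from other teams.
; A looping timer fires an object line trace along the gun's forward vector, pausing the sweep while an opposing enemy is hit and resuming otherwise.
; SetMeta assigns the owner's team, charges the player state, applies the item's material through a multicast-named event, and binds a partial refund on destruction.
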(event `Start`
  (bind (_relativerotation_roll _relativerotation_pitch) (`KismetMathLibrary.BreakRotator` (`SceneComponent.RelativeRotation` (`self.Gun`))))
  (bind (_direction _angle) (`Timeline|Timeline` :!label _label)
    (:`Update`
      (`SceneComponent.K2_SetRelativeRotation` (`self.Gun`) (`KismetMathLibrary.MakeRotator` _relativerotation_roll _relativerotation_pitch _angle) false false))))

(event `Stop`
  (goto _label :!via `Stop`))

(event `self.ReceiveBeginPlay`
  (`KismetSystemLibrary.K2_SetTimerDelegate` (delegate `Fire`) 0.2 true)
  (goto _label))

(event `Fire`
  (bind _gun (`self.Gun`))
  (bind _returnvalue (`SceneComponent.K2_GetComponentLocation` _gun))
  (bind _outhit (`KismetSystemLibrary.LineTraceSingleForObjects` :`Start` _returnvalue :`End` (+ _returnvalue (* (`SceneComponent.GetForwardVector` _gun) 1000.0)) :`ObjectTypes` (`|MakeArray` "ObjectTypeQuery8" :!type "EObjectTypeQuery Enum") :`DrawDebugType` "ForDuration"))
  (bind _asbp_base_enemy (cast `/Game/Content/Blueprints/BP_BaseEnemy` (`.HitActor` (`GameplayStatics.BreakHitResult` _outhit)))
    (:`then`
      (if (!= (`/Game/Content/Blueprints/BP_BaseEnemy.Team` _asbp_base_enemy) (`self.Team`))
        (`self.Stop`)
        (`KismetSystemLibrary.PrintString` "Fire" :!enabledstate Disabled)
        (`GameplayStatics.ApplyDamage` _asbp_base_enemy (`self.Damage`) null null "/Script/Engine.DamageType")
        (else
          (`self.Start`))))
    (:`CastFailed`
      (`self.Start`))))

(event `/Game/Content/Blueprints/BPI/BPI_SetMeta.SetMeta`
  (params (OwnedChar :type "/Game/Content/Blueprints/Char/BP_Char Object Reference") (`Selected Item` :type "/Game/Content/Blueprints/DataBase/F_Item Structure"))
  (bind (_item _team _damage _health _price _color _icon _materialinstance1 _materialinstance2) (break `/Game/Content/Blueprints/DataBase/F_Item` `Selected Item`))
  (bind _output_get (set `self.Team` (`/Game/Content/Blueprints/Char/BP_Char.Tag Team` OwnedChar)))
  (`KismetSystemLibrary.PrintString` (`KismetStringLibrary.Conv_NameToString` _output_get) :!enabledstate Disabled)
  (set `self.Price` _price)
  (`self.MULTICAST Select Material` (select `/Game/Content/Blueprints/DataBase/EN_Items` _item :`NewEnumerator0` _materialinstance1 :`NewEnumerator1` _materialinstance2))
  (bind _asbp_player_state (cast `/Game/Content/Blueprints/Char/BP_PlayerState` (`Pawn.PlayerState` OwnedChar)))
  (bind _output_get_2 (set `self.As BP Player State` _asbp_player_state))
  (set `/Game/Content/Blueprints/Char/BP_PlayerState.Money` (- (`/Game/Content/Blueprints/Char/BP_PlayerState.Money` _output_get_2) (`self.Price`)) _output_get_2)
  (add `Actor.OnDestroyed` (delegate `Add Money after Destroy`)))

(event `Add Money after Destroy`
  (params (DestroyedActor :type "Actor Object Reference"))
  (bind _as_bp_player_state (`self.As BP Player State`))
  (bind _output_get (set `/Game/Content/Blueprints/Char/BP_PlayerState.Money` (+ (`/Game/Content/Blueprints/Char/BP_PlayerState.Money` _as_bp_player_state) (/ (`self.Price`) 5)) _as_bp_player_state))
  (`KismetSystemLibrary.PrintString` (`KismetStringLibrary.Concat_StrStr` "Added Money: " (`KismetStringLibrary.Conv_IntToString` _output_get)) :!enabledstate Disabled))

(event `MULTICAST Select Material`
  (params (MI :type "MaterialInstance Object Reference"))
  (`self.Set Material` MI))

(fn `Set Material`
  (params (Item :type "MaterialInstance Object Reference"))
  (`|ExecutionSequence`
    (:`then_0`
      (`PrimitiveComponent.SetMaterial` (`self.Platform`) 0 Item))
    (:`then_1`
      (`PrimitiveComponent.SetMaterial` (`self.Gun`) 0 Item))
    (:`then_2`
      (`PrimitiveComponent.SetMaterial` (`self.Rack`) 0 Item))))

(fn `UserConstructionScript`)