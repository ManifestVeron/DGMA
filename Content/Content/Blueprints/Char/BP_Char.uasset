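; Player character with turret building: on possession it caches controller, team and player state, then spawns an owned BP_Ancient behind itself.
; While building, Tick creates one ghost turret and snaps it to surfaces using a camera trace plus a downward trace.
; Left click swaps a valid, affordable ghost for BP_TurretBase, then starts a countdown cooldown shown on TextRender.
; SERVER-prefixed events handle building; F multicasts a test turret spawn.
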(event `self.ReceivePossessed`
  (params (NewController :type "Controller Object Reference"))
  ;[1 1 1] Init
  (bind _asbp_controller (cast `/Game/Content/Blueprints/Char/BP_Controller` NewController))
  (bind _output_get (set `self.As BP Local Controller` _asbp_controller))
  (set `self.Tag Team` (`/Game/Content/Blueprints/Char/BP_Controller.Tag Team` _output_get))
  (bind _asbp_player_state (cast `/Game/Content/Blueprints/Char/BP_PlayerState` (`Controller.PlayerState` (`self.As BP Local Controller`))))
  (set `self.As BP Player State` _asbp_player_state)
  (bind _returnvalue (`|SpawnActorFromClass` "/Game/Content/Blueprints/Base/BP_Ancient.BP_Ancient_C" (`KismetMathLibrary.MakeTransform` (+ (`self.K2_GetActorLocation`) (* (`self.GetActorForwardVector`) -300.0))) "Undefined" "MultiplyWithRoot" null null))
  (message `/Game/Content/Blueprints/BPI/BPI_SetMeta.SetMeta` _returnvalue self (struct)))

(event `/Game/Content/Blueprints/BPI/BPI_ForSpawningTurret.SpawnTurret`
  (params (Enemy :type "/Game/Content/Blueprints/DataBase/F_Item Structure") (bIsBuilding :type Boolean))
  ;[1 1 1] BUILDINGS TURRET
  (`self.SERVER Spawn Turret` Enemy bIsBuilding))

(event `SERVER  BuildGhost`
  (bind _returnvalue (`self.GetTransform`))
  ;[1 1 1] BUILDINGS TURRET
  (`/Engine/EditorBlueprintResources/StandardMacros.DoOnce` false :!label _label
    (:`Completed`
      (bind _returnvalue_2 (`|SpawnActorFromClass` "/Game/Content/Blueprints/Turret/BP_TurretGhost.BP_TurretGhost_C" (`KismetMathLibrary.MakeTransform` (.location _returnvalue) (`KismetMathLibrary.MakeRotator` (.roll (.rotation _returnvalue)) (.pitch (.rotation _returnvalue)) (- (.yaw (.rotation _returnvalue)) 90.0)) (.scale _returnvalue)) "Undefined" "MultiplyWithRoot" null null))
      (set `self.BP_TurretGhost` _returnvalue_2))))

(event `SERVER Reset Build Ghost`
  ;[1 1 1] BUILDINGS TURRET
  (goto _label :!via `Reset`))

(event `SERVER Spawn Turret`
  (params (SelectedTurret :type "/Game/Content/Blueprints/DataBase/F_Item Structure") (IsBuilding :type Boolean))
  ;[1 1 1] BUILDINGS TURRET
  (bind _output_get (set `self.Selected Turret` SelectedTurret))
  (set `self.TurretPrice` (`.Price_24_47A47C5944EA9E422103CAB5B97254E1` (break `/Game/Content/Blueprints/DataBase/F_Item` _output_get)))
  (set `self.bIsBuilding` IsBuilding))

(event `self.ReceiveTick`
  (params (DeltaSeconds :type "Float (single-precision)"))
  ;[1 1 1] BUILDINGS TURRET
  (if (`self.bIsBuilding`)
    (`|ExecutionSequence`
      (:`then_0`
        (`self.SERVER  BuildGhost`))
      (:`then_1`
        (`self.SERVER Moving Ghost`)))))

(event `SERVER Moving Ghost`
  ;[1 1 1] BUILDINGS TURRET
  (bind _out_hit_location (`self.BuildTrace`))
  (`self.K2_SetActorLocation` (`self.BP_TurretGhost`) _out_hit_location false false))

(event `Key|LeftMouseButton`
  (params (Key :type "Key Structure"))
  ;[1 1 1] BUILDINGS TURRET
  (:`Pressed`
    (`self.SERVER SpawnSelectedTurret`)))

(event `SERVER SpawnSelectedTurret`
  (bind _bp_turretghost (`self.BP_TurretGhost`))
  ;[1 1 1] BUILDINGS TURRET
  (`/Engine/EditorBlueprintResources/StandardMacros.IsValid` _bp_turretghost
    (:`Is Valid`
      (if (and (`self.bIsBuilding`) (`/Game/Content/Blueprints/Turret/BP_TurretGhost.bIsSpawn` _bp_turretghost) (`self.bIsNoСooldown`) (>= (`/Game/Content/Blueprints/Char/BP_PlayerState.Money` (`self.As BP Player State`)) (`self.TurretPrice`)))
        (set `self.bIsBuilding` false)
        (bind _returnvalue (`|SpawnActorFromClass` "/Game/Content/Blueprints/Turret/BP_TurretBase.BP_TurretBase_C" (`self.GetTransform` (`self.BP_TurretGhost`)) "Undefined" "MultiplyWithRoot" null null))
        (message `/Game/Content/Blueprints/BPI/BPI_SetMeta.SetMeta` _returnvalue self (`self.Selected Turret`))
        (`self.K2_DestroyActor` (`self.BP_TurretGhost`))
        (bind _returnvalue_2 (`KismetSystemLibrary.K2_SetTimerDelegate` (delegate `Cull Down`) 1.0 true))
        (`self.SERVER Reset Build Ghost`)))))

(event `Cull Down`
  ;[1 1 1] BUILDINGS TURRET
  (`self.SERVER Cooldown`))

(event `SERVER Cooldown`
  (bind _culldown (`self.CullDown`))
  ;[1 1 1] BUILDINGS TURRET
  (if (> (`self.CullDown`) 0)
    (set `self.bIsNoСooldown` false)
    (`/Engine/EditorBlueprintResources/StandardMacros.DecrementInt` _culldown
      (:`  `
        (`TextRenderComponent.K2_SetText` (`self.TextRender`) (`KismetTextLibrary.Conv_IntToText` _culldown))))
    (else
      (`KismetSystemLibrary.K2_ClearAndInvalidateTimerHandle` (stale `SERVER SpawnSelectedTurret` _returnvalue_2))
      (set `self.bIsNoСooldown` true)
      (bind _output_get (set `self.CullDown` 5))
      (`TextRenderComponent.K2_SetText` (`self.TextRender`) (`KismetTextLibrary.Conv_IntToText` _output_get)))))

(event `Key|F`
  (params (Key :type "Key Structure"))
  ;[1 1 1] Check RPC
  (:`Pressed`
    (`self.SERVER SpawnTEST`)))

(event `SERVER SpawnTEST`
  ;[1 1 1] Check RPC
  (`self.MULTICAST SpawnTEST`))

(event `MULTICAST SpawnTEST`
  (bind _returnvalue (`self.GetTransform`))
  ;[1 1 1] Check RPC
  (`|SpawnActorFromClass` "/Game/Content/Blueprints/Turret/BP_TurretBase.BP_TurretBase_C" (`KismetMathLibrary.MakeTransform` (+ (.location _returnvalue) (500.0 0.0 0.0)) (`KismetMathLibrary.MakeRotator` (.roll (.rotation _returnvalue)) (.pitch (.rotation _returnvalue)) (- (.yaw (.rotation _returnvalue)) 90.0)) (.scale _returnvalue)) "Undefined" "MultiplyWithRoot" null null))

(fn `BuildTrace`
  (returns (`Out Hit Location` :type "Vector Structure"))
  (locals (`Actors to Ignore` :type "Array of /Game/Content/Blueprints/Turret/BP_TurretGhost Object Reference"))
  (bind _followcamera (`self.FollowCamera`))
  (bind _returnvalue (`SceneComponent.K2_GetComponentLocation` _followcamera))
  (bind _output_get (set `local.Actors to Ignore` (`|MakeArray` (`self.BP_TurretGhost`))))
  (bind (_outhit _returnvalue_2) (`KismetSystemLibrary.LineTraceSingle` _returnvalue (+ (* (`SceneComponent.GetForwardVector` _followcamera) 1000.0) _returnvalue) "TraceTypeQuery1" false _output_get))
  (if _returnvalue_2
    (bind (_bblockinghit _binitialoverlap _time _distance _location _impactpoint _normal _impactnormal _physmat _hitactor _hitcomponent _hitbonename _bonename _hititem _elementindex _faceindex _tracestart _traceend) (`GameplayStatics.BreakHitResult` _outhit))
    (bind _outhit_2 (`KismetSystemLibrary.LineTraceSingle` (+ _location (0.0 0.0 500.0)) (- _location (0.0 0.0 50.0)) "TraceTypeQuery1" false (`local.Actors to Ignore`)))
    (return (`.Location` (`GameplayStatics.BreakHitResult` _outhit_2)))
    (else
      (bind _outhit_3 (`KismetSystemLibrary.LineTraceSingle` _traceend (- _traceend (0.0 0.0 500.0)) "TraceTypeQuery1" false (`local.Actors to Ignore`)))
      (return (`.Location` (`GameplayStatics.BreakHitResult` _outhit_3))))))

(fn `UserConstructionScript`)