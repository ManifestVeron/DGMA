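; BP_Controller is the player controller that handles team-based spawning and the local player's UI.
; On BeginPlay the local controller shows team selection and money widgets and creates a hidden construction menu, which E toggles through a FlipFlop.
; SERVERSpawnPlayer stores the chosen team tag and asks BP_GameMode to spawn the player.
; It then adds the default Enhanced Input mapping context if the passed controller is local.
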(event `self.ReceiveBeginPlay`
  (if (`self.IsLocalPlayerController`)
    (bind _returnvalue (`|CreateWidget` "/Game/Content/Blueprints/Widgets/BPW_SelectTeam.BPW_SelectTeam_C"))
    (`UserWidget.AddToViewport` _returnvalue 0)
    (`self.InitUMG`)))

(event `SERVER Spawn Player`
  (params (`Tag Team` :type Name) (BP_PlayerController :type "/Game/Blueprints/Char/BP_Controller Object Reference"))
  (bind _output_get (set `self.Tag Team` `Tag Team`))
  (bind _asbp_game_mode (cast `/Game/Content/Blueprints/BP_GameMode` (`GameplayStatics.GetGameMode`)))
  (`/Game/Content/Blueprints/BP_GameMode.SpawnPlayer` _asbp_game_mode _output_get self)
  (`self.InitLocalPlayerController` BP_PlayerController))

(event `InitLocalPlayerController`
  (params (LocalPlayerController :type "/Game/Blueprints/Char/BP_Controller Object Reference"))
  (if (`self.IsLocalPlayerController` LocalPlayerController)
    (`EnhancedInputSubsystemInterface.AddMappingContext` (pcsubsystem `EnhancedInputLocalPlayerSubsystem` LocalPlayerController) "/Game/ExternContent/ThirdPerson/Input/IMC_Default.IMC_Default" 0 (struct))))

(event `InitUMG`
  (if (`self.IsLocalPlayerController`)
    (bind _returnvalue (`|CreateWidget` "/Game/Content/Blueprints/Widgets/BPW_Money.BPW_Money_C"))
    (`UserWidget.AddToViewport` _returnvalue 0)
    (bind _returnvalue_2 (`|CreateWidget` "/Game/Content/Blueprints/Widgets/BPW_ConstructionMenu.BPW_ConstructionMenu_C" self))
    (`UserWidget.AddToViewport` _returnvalue_2 0)
    (`Widget.SetVisibility` _returnvalue_2 "Hidden")))

(event `Key|E`
  (params (Key :type "Key Structure"))
  (:`Pressed`
    (`/Engine/EditorBlueprintResources/StandardMacros.FlipFlop`
      (:`A`
        (`Widget.SetVisibility` (stale `InitUMG` _returnvalue_2) "Visible"))
      (:`B`
        (`Widget.SetVisibility` (stale `InitUMG` _returnvalue_2) "Hidden")))))

(fn `UserConstructionScript`)