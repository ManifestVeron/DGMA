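; BP_PlayerState is a player state that gives the player passive income that speeds up over time.
; A looping timer polls until the pawn casts to BP_Char, caches that reference, then clears itself and starts two looping timers.
; One regularly adds AddMoney times Coefficient to Money, while a slower one increments Coefficient, so earnings grow the longer the timers run.
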(event `self.ReceiveBeginPlay`
  (bind _returnvalue (`KismetSystemLibrary.K2_SetTimerDelegate` (delegate `CheckPosses`) 1.0 true)))

(event `CheckPosses`
  (bind _asbp_char (cast `/Game/Content/Blueprints/Char/BP_Char` (`self.GetPawn`)))
  (set `self.As BP Char` _asbp_char)
  (`KismetSystemLibrary.K2_SetTimerDelegate` (delegate `Add Money`) 2.0 true)
  (`KismetSystemLibrary.K2_ClearAndInvalidateTimerHandle` (stale `self.ReceiveBeginPlay` _returnvalue))
  (`KismetSystemLibrary.K2_SetTimerDelegate` (delegate `Increase in ratio over time`) 20.0 true))

(event `Increase in ratio over time`
  (`/Engine/EditorBlueprintResources/StandardMacros.IncrementInt` (`self.Coefficient`)
    (:`  `
      (`KismetSystemLibrary.PrintString` "Add Coefficent  +1" :!enabledstate Disabled))))

(event `Add Money`
  (set `self.Money` (+ (`self.Money`) (* (`self.AddMoney`) (`self.Coefficient`)))))

(fn `UserConstructionScript`)