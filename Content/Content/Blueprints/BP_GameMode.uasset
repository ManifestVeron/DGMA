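; Game mode blueprint for a team-based match, handling player spawning and the end of play.
; SpawnPlayer picks a random PlayerStart tagged with the team, spawns a BP_Char there and has the given controller possess it.
; SetMeta takes a character, prints that its team lost, then destroys the controlled pawn of every player controller to end play.
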(event `self.ReceiveBeginPlay`)

(event `/Game/Content/Blueprints/BPI/BPI_SetMeta.SetMeta`
  (params (OwnedChar :type "/Game/Content/Blueprints/Char/BP_Char Object Reference") (`Selected Item` :type "/Game/Content/Blueprints/DataBase/F_Item Structure"))
  (`KismetSystemLibrary.PrintString` (`KismetStringLibrary.Concat_StrStr` "TEAM  " (`KismetStringLibrary.Conv_NameToString` (`/Game/Content/Blueprints/Char/BP_Char.Tag Team` OwnedChar)) "  LOST. END PLAY") true true (struct :`R` 1.0 :`A` 1.0) 5.0)
  (for _index (range (`GameplayStatics.GetNumPlayerControllers`))
    (`self.K2_DestroyActor` (`Controller.K2_GetPawn` (`GameplayStatics.GetPlayerController` _index)))))

(fn `SpawnPlayer`
  (params (`Team Tag` :type Name) (`Player Controller` :type "/Game/Content/Blueprints/Char/BP_Controller Object Reference"))
  (bind _outactors (`GameplayStatics.GetAllActorsOfClassWithTag` "/Script/Engine.PlayerStart" `Team Tag`))
  (bind _returnvalue (`|SpawnActorFromClass` "/Game/Content/Blueprints/Char/BP_Char.BP_Char_C" (`self.GetTransform` (`KismetArrayLibrary.Array_Random` _outactors)) "Undefined" "MultiplyWithRoot" null null))
  (bind _output_get (set `self.BP Char` _returnvalue))
  (`Controller.Possess` `Player Controller` _output_get))

(fn `UserConstructionScript`)